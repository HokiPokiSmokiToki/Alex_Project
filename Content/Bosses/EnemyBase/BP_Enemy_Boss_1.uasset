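; Boss enemy character with a health bar, a melee attack and a death sequence.
; On spawn it adds a boss health widget to the viewport and refreshes the bar from Health every Tick.
; Attack plays a montage guarded by IsAttacking, using its notify to sphere-trace forward from the mesh for pawns and apply damage.
; Incoming damage lowers Health; at zero or below, movement stops, mesh physics turns on and a death montage plays.
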(event `self.ReceiveTick`
  (params (DeltaSeconds :type "Float (single-precision)"))
  (`ProgressBar.SetPercent` (`/Game/Bosses/EnemyBase/WB_Boss_Health.HealthBar` (`self.HealthUI`)) (/ (`self.Health`) 1000.0)))

(event `self.ReceiveBeginPlay`
  (bind _returnvalue (`|CreateWidget` "/Game/Bosses/EnemyBase/WB_Boss_Health.WB_Boss_Health_C"))
  (`UserWidget.AddToViewport` _returnvalue 0)
  (set `self.HealthUI` _returnvalue))

(event `/Game/Bosses/EnemyBase/BPI_BossFight.Attack`
  (bind _mesh (`self.Mesh`))
  (bind _returnvalue (`SceneComponent.K2_GetComponentLocation` _mesh))
  ; Attack
  (if (not (`self.IsAttacking?`))
    (`|PlayMontage` (`self.Mesh`) "/Game/BattleWizardPolyart/Animations/Attack01Anim_Montage.Attack01Anim_Montage"
      (:`then`
        (set `self.IsAttacking?` true))
      (:`OnCompleted`
        (set `self.IsAttacking?` false))
      (:`OnNotifyBegin`
        (bind (_outhit _returnvalue_2) (`KismetSystemLibrary.SphereTraceSingleForObjects` :`Start` _returnvalue :`End` (+ _returnvalue (* 500.0 (`KismetMathLibrary.GetForwardVector` (`SceneComponent.K2_GetComponentRotation` _mesh)))) :`Radius` 50.0 :`ObjectTypes` (`|MakeArray` "ObjectTypeQuery3" :!type "EObjectTypeQuery Enum") :`DrawDebugType` "ForDuration"))
        (if _returnvalue_2
          (`GameplayStatics.ApplyDamage` (`.HitActor` (`GameplayStatics.BreakHitResult` _outhit)) 10.0))))))

(event `self.ReceiveAnyDamage`
  (params (Damage :type "Float (single-precision)") (DamageType :type "DamageType Object Reference") (InstigatedBy :type "Controller Object Reference") (DamageCauser :type "Actor Object Reference"))
  ; Checks health of boss and plays anim when health == 0
  (set `self.Health` (- (`self.Health`) Damage))
  (if (<= (`self.Health`) 0.0)
    (`CharacterMovementComponent.DisableMovement` (`self.CharacterMovement`))
    (`PrimitiveComponent.SetSimulatePhysics` (`self.Mesh`) true)
    (`|PlayMontage` (`self.Mesh`) "/Game/BattleWizardPolyart/Animations/DieAnim_Montage.DieAnim_Montage")))

(fn `UserConstructionScript`
  (`parent.UserConstructionScript`))