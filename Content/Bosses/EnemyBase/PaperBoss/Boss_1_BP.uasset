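; Paper2D slime boss that chases the player and shoots at them, with an on-screen health bar.
; Tick refreshes the bar, sets the move flipbook and reissues AIMoveTo toward the player.
; PawnSensing spawns a bullet on seeing the player, gated by a two-second cooldown.
; Damage shows a number widget, sets the hit flipbook, lowers health and, at zero, disables movement and flags Dead.
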(event `self.ReceiveAnyDamage`
  (params (Damage :type "Float (single-precision)") (DamageType :type "DamageType Object Reference") (InstigatedBy :type "Controller Object Reference") (DamageCauser :type "Actor Object Reference"))
  ;[0.7979 1 0 0.5] On take damage show damage number on screen and play flipbook anim
  (bind _returnvalue (`|CreateWidget` "/Game/UserInterface/Misc/W_DamageNumber.W_DamageNumber_C" null self Damage))
  (`UserWidget.AddToViewport` _returnvalue 0)
  (`PaperFlipbookComponent.SetFlipbook` (`self.Sprite`) "/Game/Bosses/EnemyBase/Sprites/Hit/Slime_Hit_FB.Slime_Hit_FB")
  ;[0.6871 1 0 0.5] Checks if health of boss is above 0 if not disables movement.
  (set `self.Health` (- (`self.Health`) Damage))
  (if (<= (`self.Health`) 0.0)
    (`CharacterMovementComponent.DisableMovement` (`self.CharacterMovement`))
    (set `self.Dead?` true)))

(event `self.ReceiveTick`
  (params (DeltaSeconds :type "Float (single-precision)"))
  ;[0.8224 1 0 0.5] Sets inital health and continuosly updates it every tick, also sets flipbook
  (`ProgressBar.SetPercent` (`/Game/Bosses/EnemyBase/WB_Boss_Health.HealthBar` (`self.Health UI`)) (/ (`self.Health`) 1000.0))
  (`PaperFlipbookComponent.SetFlipbook` (`self.Sprite`) "/Game/Bosses/EnemyBase/Sprites/Move/Slime_Move_FB.Slime_Move_FB")
  ;[0.5428 1 0 0.5] Chase player
  (`|AIMoveTo` self (`self.K2_GetActorLocation` (`GameplayStatics.GetPlayerCharacter` 0)) null 50.0))

(event `self.ReceiveBeginPlay`
  ;[0.874 1 0 0.5] Adds boss health widget to viewport
  (bind _returnvalue (`|CreateWidget` "/Game/Bosses/EnemyBase/WB_Boss_Health.WB_Boss_Health_C"))
  (`UserWidget.AddToViewport` _returnvalue 0)
  (set `self.Health UI` _returnvalue))

(event `self.PawnSensing.OnSeePawn`
  (params (Pawn :type "Pawn Object Reference"))
  ;[0.5442 1 0.204 0.5] Shoot projectile at player
  (cast `/Game/Character/BluePrints/BP_TopDown_Char` Pawn)
  (if (not (`self.Is Attacking?`))
    (`|SpawnActorFromClass` "/Game/Bosses/EnemyBase/PaperBoss/EnemyBullet_BP.EnemyBullet_BP_C" (`self.GetTransform`) "AdjustIfPossibleButAlwaysSpawn" "MultiplyWithRoot" null null)
    (set `self.Is Attacking?` true)
    (`KismetSystemLibrary.Delay` 2.0)
    (set `self.Is Attacking?` false)))

(fn `UserConstructionScript`)