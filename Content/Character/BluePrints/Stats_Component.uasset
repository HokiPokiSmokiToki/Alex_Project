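; Stats component that stores named numeric character stats, such as Health, in a map.
; AlterStat adds a change to an existing stat and returns its value and depletion state, printing an error for unknown names.
; QueryStat reads a value by name.
; OnDamaged subtracts damage from Health, but its binding to the owner's damage event is unconnected, so the component never binds it itself.
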(event `OnDamaged`
  (params (DamagedActor :type "Actor Object Reference") (Damage :type "Float (single-precision)") (DamageType :type "DamageType Object Reference") (InstigatedBy :type "Controller Object Reference") (DamageCauser :type "Actor Object Reference"))
  (`self.AlterStat` "Health" (* Damage -1.0)))

(fn `AlterStat`
  (params (Stat :type String) (Change :type "Float (double-precision)"))
  (returns (StatDepleted :type Boolean) (CurrentValue :type "Float (double-precision)"))
  (bind _stats (`self.Stats`))
  (bind _stat (`local.Stat`))
  (bind (_value _returnvalue) (`BlueprintMapLibrary.Map_Find` (`self.Stats`) Stat))
  (bind _value_2 (`BlueprintMapLibrary.Map_Find` _stats _stat))
  (if _returnvalue
    (`BlueprintMapLibrary.Map_Add` _stats _stat (+ _value Change))
    (return (<= _value_2 0.0) _value_2)
    (else
      (`KismetSystemLibrary.PrintString` "No Valid Stat With Name"))))

(fn `QueryStat`
  (params (Stat :type String))
  (returns (Value :type "Float (double-precision)"))
  (return (`BlueprintMapLibrary.Map_Find` (`self.Stats`) Stat)))