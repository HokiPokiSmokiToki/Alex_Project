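; BP_Gate_1 is a camp gate that sends the top-down player character into Level_1.
; Its trigger overlap casts to BP_TopDown_Char and branches on a LevelComplete flag.
; If the level is complete, it only prints debug text.
; Otherwise it plays a camera shutter sound, shows a Fade_WB fade widget and opens the level by name after a short delay.
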(event `self.Trigger.OnComponentBeginOverlap`
  (params (OverlappedComponent :type "PrimitiveComponent Object Reference") (OtherActor :type "Actor Object Reference") (OtherComp :type "PrimitiveComponent Object Reference") (OtherBodyIndex :type Integer) (bFromSweep :type Boolean) (SweepResult :type "HitResult Structure (by ref)"))
  (cast `/Game/Character/BluePrints/BP_TopDown_Char` OtherActor)
  (`KismetSystemLibrary.PrintString` "L1")
  (if (`self.Level_Complete`)
    (`KismetSystemLibrary.PrintString` "Complete")
    (else
      (`GameplayStatics.PlaySound2D` "/Engine/VREditor/Sounds/UI/Camera_Shutter.Camera_Shutter" 1.0 1.0 0.0 null null)
      (bind _returnvalue (`|CreateWidget` "/Game/Levels/UI/Fade_WB.Fade_WB_C"))
      (`UserWidget.AddToViewport` _returnvalue 0)
      (`/Game/Levels/UI/Fade_WB.Fade_Anim` _returnvalue)
      (`KismetSystemLibrary.Delay` 0.5)
      (`GameplayStatics.OpenLevel` "Level_1"))))

(fn `UserConstructionScript`)