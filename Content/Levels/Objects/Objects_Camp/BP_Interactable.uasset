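; BP_Interactable is a camp level object that opens and closes a shop UI when interacted with.
; A Sphere component's overlap events show and hide a Widget component that serves as the icon.
; The Interact event toggles on a boolean, either creating a new Shop_WB and adding it to the viewport or hiding the current one.
; Each opening creates a fresh widget, as closing only hides the previous one.
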(event `self.Sphere.OnComponentBeginOverlap`
  (params (OverlappedComponent :type "PrimitiveComponent Object Reference") (OtherActor :type "Actor Object Reference") (OtherComp :type "PrimitiveComponent Object Reference") (OtherBodyIndex :type Integer) (bFromSweep :type Boolean) (SweepResult :type "HitResult Structure (by ref)"))
  ;[0 1 0.07177] Switch between visibility of icon
  (`SceneComponent.SetVisibility` (`self.Widget`) true false))

(event `self.Sphere.OnComponentEndOverlap`
  (params (OverlappedComponent :type "PrimitiveComponent Object Reference") (OtherActor :type "Actor Object Reference") (OtherComp :type "PrimitiveComponent Object Reference") (OtherBodyIndex :type Integer))
  ;[0 1 0.07177] Switch between visibility of icon
  (`SceneComponent.SetVisibility` (`self.Widget`) false false))

(event `/Game/UserInterface/Interactions/Interact_Interface.Interact`
  ;[0.1232 1 0 0.5] Creates shop WB on interaction, then Hides it if interacted again.
  (if (`self.Interact?`)
    (set `self.Interact?` false)
    (bind _returnvalue (`|CreateWidget` "/Game/Bosses/ShopKeeper/Shop_WB.Shop_WB_C"))
    (`UserWidget.AddToViewport` _returnvalue 0)
    (else
      (set `self.Interact?` true)
      (`Widget.SetVisibility` _returnvalue "Hidden"))))

(fn `UserConstructionScript`)